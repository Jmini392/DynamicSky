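; BP_DynamicSky is a sky actor that sets sun, moon and atmosphere from a TimeOfDay value, entirely in the Construction Script.
; Sun and moon pitch are remapped around DawnTime and DuskTime; the second, pre-dawn moon rotation always overwrites the evening one.
; IsDayTime and IsNightTime checks toggle each light's visibility.
; Night applies configurable moonlight and atmosphere scattering settings, while day restores hardcoded scattering values.
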(fn `HandleNightSettings`
  (bind _moondirectionallight (`self.MoonDirectionalLight`))
  (bind _skyatmosphere (`self.SkyAtmosphere`))
  (bind _skyatmosphere_2 (`self.SkyAtmosphere`))
  (if (`self.IsNightTime`)
    (`|ExecutionSequence`
      (:`then_0`
        (`LightComponent.SetIntensity` _moondirectionallight (`self.MoonLightIntensity`))
        (`LightComponent.SetLightColor` _moondirectionallight (`self.MoonLightColor`) true)
        (`DirectionalLightComponent.SetLightSourceAngle` _moondirectionallight (`self.MoonLightSourceAngle`))
        (`LightComponent.SetTemperature` _moondirectionallight (`self.MoonLightTemperature`)))
      (:`then_1`
        (`SkyAtmosphereComponent.SetRayleighScattering` _skyatmosphere_2 (`self.NightTimeRayleighScattering`))
        (`SkyAtmosphereComponent.SetMultiScatteringFactor` _skyatmosphere_2 (`self.NightTimeMultiScattering`))))
    (else
      (`SkyAtmosphereComponent.SetRayleighScattering` _skyatmosphere (struct :`R` 0.174647 :`G` 0.40724 :`B` 1.0 :`A` 1.0))
      (`SkyAtmosphereComponent.SetMultiScatteringFactor` _skyatmosphere 1.0))))

(fn `HandleSunMoonRotation`
  (`SceneComponent.K2_SetWorldRotation` (`self.SunDirectionalLight`) (`KismetMathLibrary.MakeRotator` 0.0 (`KismetMathLibrary.MapRangeUnclamped` (`self.TimeOfDay`) (`self.DawnTime`) (`self.DuskTime`) 0.0 -180.0)) false false)
  (`SceneComponent.K2_SetWorldRotation` (`self.MoonDirectionalLight`) (`KismetMathLibrary.MakeRotator` 0.0 (`KismetMathLibrary.MapRangeUnclamped` (`self.TimeOfDay`) (+ (`self.DuskTime`) 0.2) 24.0 -180.0 -90.0)) false false)
  (`SceneComponent.K2_SetWorldRotation` (`self.MoonDirectionalLight`) (`KismetMathLibrary.MakeRotator` 0.0 (`KismetMathLibrary.MapRangeUnclamped` (`self.TimeOfDay`) 0.0 (- (`self.DawnTime`) 0.2) -90.0 0.0)) false false))

(fn `HandleVisibility`
  (`SceneComponent.SetVisibility` (`self.SunDirectionalLight`) (`self.IsDayTime`) false)
  (`SceneComponent.SetVisibility` (`self.MoonDirectionalLight`) (`self.IsNightTime`) false))

(fn `UserConstructionScript`
  (`|ExecutionSequence`
    (:`then_1`
      (`self.HandleSunMoonRotation`))
    (:`then_2`
      (`self.HandleVisibility`))
    (:`then_3`
      (`self.HandleNightSettings`))))